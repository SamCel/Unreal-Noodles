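; BasicBullet is a shmup projectile actor that acts as either a bullet or an accelerating missile.
; FireProjectile loads transform, direction, speed, lifetime and other data, then activates it.
; Tick toggles visuals by type, moves it forward and hands it to the game instance's BulletManager via DisableMe on expiry.
; Seeking missiles have no movement logic here, Damage is only stored, and overlap only prints debug text.
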(event `self.ReceiveActorBeginOverlap`
  (params (OtherActor :type "Actor Object Reference"))
  (`KismetSystemLibrary.PrintString` "i ded"))

(event `self.ReceiveTick`
  (params (DeltaSeconds :type "Float (single-precision)"))
  (bind _missile (`self.Missile`))
  (bind _bullet (`self.Bullet`))
  (set `self.deltaTime` DeltaSeconds)
  (if (`self.IsActive`)
    (if (`ActorComponent.IsActive` (`self.ParticleSystem`))
      (switch `ProjectileType` (`self.Type`)
        (:`PT_Bullet`
          (set `self.Part` (`self.ParticleSystem`))
          (`SceneComponent.SetVisibility` _bullet true true)
          (`SceneComponent.SetVisibility` _missile false true))
        (:`PT_Missile`
          (set `self.Part` (`self.ParticleSystem1`))
          (`SceneComponent.SetVisibility` _bullet false true)
          (`SceneComponent.SetVisibility` _missile true true)))
      (if (>= (`self.LifeTime`) (`self.MaxLifetime`))
        (`/Game/Blueprints/BulletManager.DisableMe` (`self.BulletManager`) self)
        (`ActorComponent.Deactivate` (`self.Part`))
        (else
          (bind _output_get (set `self.LifeTime` (+ (`self.LifeTime`) (`self.deltaTime`))))
          (switch `ProjectileType` (`self.Type`)
            (:`PT_Bullet`
              (`self.K2_AddActorWorldOffset` (* (`self.travelForwardDirection`) (* (`self.deltaTime`) (`self.speed`)))))
            (:`PT_Missile`
              (if (not (> (`self.speed`) (`self.maxSpeed`)))
                (set `self.speed` (+ (`self.speed`) (`self.acceleration`))))
              (if (not (`self.seeking`))
                (`self.K2_AddActorWorldOffset` (* (`self.travelForwardDirection`) (* (`self.deltaTime`) (`self.speed`)))))))))
      (else
        (`ActorComponent.Activate` (`self.Part`) false)))))

(event `self.ReceiveBeginPlay`
  (bind _asshmup_game_instance (cast `/Game/Blueprints/ShmupGameInstance` (`GameplayStatics.GetGameInstance`))
    (:`then`
      (bind _manager (`/Game/Blueprints/ShmupGameInstance.GetManager` _asshmup_game_instance))
      (set `self.BulletManager` _manager)
      (set `self.Part` (`self.ParticleSystem`)))
    (:`CastFailed`
      (`KismetSystemLibrary.PrintText` "Failed to find BulletManager!\n"))))

(fn `FireProjectile`
  (params (Data :type "BulletData Structure"))
  (bind (_origin _traveldirection _bullettype _maxlife _maxspeed _initialspeed _damage _size _seeking) (break `BulletData` Data))
  (`self.K2_SetActorTransform` _origin)
  (set `self.travelForwardDirection` _traveldirection)
  (set `self.MaxLifetime` _maxlife)
  (set `self.Type` _bullettype)
  (set `self.maxSpeed` _maxspeed)
  (set `self.speed` _initialspeed)
  (set `self.damage` _damage)
  (`self.SetActorScale3D` (* (`self.GetActorScale3D`) _size))
  (set `self.seeking` _seeking)
  (set `self.IsActive` true))

(fn `UserConstructionScript`)