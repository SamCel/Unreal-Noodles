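; DancerFire is a shmup weapon component that fires projectiles from several local-space origins while FireWeap1 is set.
; BeginPlay gets the BulletManager from ShmupGameInstance and builds four hardcoded weapon presets, equipping DoubleMinigun.
; Tick accumulates a cooldown, then rotates each origin into world space and requests randomly scattered shots from the manager per the current weapon's data.
; Each origin also draws a debug sphere when it fires.
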(event `self.ReceiveTick`
  (params (DeltaSeconds :type "Float (single-precision)"))
  (bind (_bulletdata _timebetweenshots _shotstofire _scatter) (break `WeaponData` (`self.currentWeapon1`)))
  (bind (_origin _traveldirection _bullettype _maxlife _maxspeed _initialspeed _damage _size _seeking) (break `BulletData` _bulletdata))
  (if (`self.FireWeap1`)
    (if (> (`self.fireTime`) _timebetweenshots)
      (set `self.fireTime` 0.0)
      (for _array_element (`self.Default Fire Origins`)
        (bind _returnvalue (+ (`self.K2_GetComponentLocation`) (`KismetMathLibrary.GreaterGreater_VectorRotator` _array_element (`self.K2_GetComponentRotation`))))
        (`KismetSystemLibrary.DrawDebugSphere` _returnvalue 30.0 12 (struct :`R` 1.0 :`B` 0.945804 :`A` 1.0) 0.0 1.0)
        (for _ (range (+ (`KismetMathLibrary.FTrunc` _shotstofire) 1))
          (`/Game/Blueprints/BulletManager.FireProjectile` (`self.BulletManager`) (make `BulletData` (`KismetMathLibrary.MakeTransform` _returnvalue (`self.K2_GetComponentRotation`)) (`KismetMathLibrary.RandomUnitVectorInEllipticalConeInDegrees` (`KismetMathLibrary.GetForwardVector` (`self.K2_GetComponentRotation`)) _scatter _scatter) _bullettype _maxlife _maxspeed _initialspeed _damage _size _seeking))))
      (else
        (set `self.fireTime` (+ (`self.fireTime`) (`GameplayStatics.GetWorldDeltaSeconds`)))))))

(event `self.ReceiveBeginPlay`
  (bind _asshmup_game_instance (cast `/Game/Blueprints/ShmupGameInstance` (`GameplayStatics.GetGameInstance`))
    (:`then`
      (bind _manager (`/Game/Blueprints/ShmupGameInstance.GetManager` _asshmup_game_instance))
      (set `self.BulletManager` _manager)
      (set `self.DoubleMissile` (make `WeaponData` (make `BulletData` (struct) (0.0 0.0 0.0) "PT_Missile" 10.0 3500.0 0.0 0.0 4.0) 0.45 10.0 15.0))
      (set `self.DoubleMinigun` (make `WeaponData` (make `BulletData` (struct) (0.0 0.0 0.0) "PT_Bullet" 2.0 3500.0 3000.0 0.0 2.0) 0.025 1.0 2.0))
      (set `self.SingleShotgun` (make `WeaponData` (make `BulletData` (struct) (0.0 0.0 0.0) "PT_Bullet" 5.0 3500.0 3000.0 0.0 2.0) 0.25 70.0 30.0))
      (set `self.BIGBOBI` (make `WeaponData` (make `BulletData` (struct) (0.0 0.0 0.0) "PT_Missile" 20.0 2000.0 0.0 0.0 30.0) 2.0))
      (set `self.currentWeapon1` (`self.DoubleMinigun`)))
    (:`CastFailed`
      (`KismetSystemLibrary.PrintText` "Hello"))))