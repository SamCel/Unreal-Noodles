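; BulletManager is an object pool for BasicBullet projectiles, avoiding spawning an actor per shot.
; BeginPlay pre-spawns the bullets at its own transform and parks them with DisableMe, which turns off collision, visibility and tick and resets their state.
; FireProjectile wakes the first inactive bullet, moves it to the requested origin, launches it with the supplied data and returns it.
; When all are active, it recycles the one with the longest LifeTime.
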(event `self.ReceiveBeginPlay`
  (for _ (range 251)
    (bind _returnvalue (`|SpawnActorFromClass` "/Game/Blueprints/BasicBullet.BasicBullet_C" (`self.K2_GetComponentToWorld`) "AlwaysSpawn" "OverrideRootScale" null null))
    (`KismetArrayLibrary.Array_Add` (`self.BulletArray`) _returnvalue)
    (`self.DisableMe` _returnvalue)))

(fn `DisableMe`
  (params (BulletToDisable :type "/Game/Blueprints/BasicBullet Object Reference"))
  (`Actor.SetActorEnableCollision` BulletToDisable false)
  (`Actor.SetActorHiddenInGame` BulletToDisable true)
  (`Actor.SetActorTickEnabled` BulletToDisable false)
  (`Actor.K2_SetActorLocation` BulletToDisable (`self.K2_GetComponentLocation`) false false)
  (`Actor.SetActorScale3D` BulletToDisable (1.0 1.0 1.0))
  (set `/Game/Blueprints/BasicBullet.IsActive` false BulletToDisable)
  (set `/Game/Blueprints/BasicBullet.LifeTime` 0.0 BulletToDisable))

(fn `FireProjectile`
  (params (InputData :type "BulletData Structure"))
  (returns (FiredBullet :type "/Game/Blueprints/BasicBullet Object Reference"))
  (locals (NewLocalVar_0 :type "Float (double-precision)" :default 0.0) (CurrentBulletInArray :type "/Game/Blueprints/BasicBullet Object Reference") (bulletData :type "BulletData Structure"))
  (bind _currentbulletinarray (`local.CurrentBulletInArray`))
  (bind _oldestbullet (`self.OldestBullet`))
  (bind _lifetime (`/Game/Blueprints/BasicBullet.LifeTime` (`local.CurrentBulletInArray`)))
  (set `local.bulletData` InputData)
  (for _array_element (`self.BulletArray`)
    (bind _output_get (set `local.CurrentBulletInArray` _array_element))
    (if (`/Game/Blueprints/BasicBullet.IsActive` _output_get)
      (if (> _lifetime (`self.LongestLifetime`))
        (set `self.OldestBullet` (`local.CurrentBulletInArray`))
        (set `self.LongestLifetime` _lifetime))
      (else
        (set `self.BulletFound` true)
        (set `self.LongestLifetime` 0.0)
        (`Actor.SetActorHiddenInGame` _currentbulletinarray false)
        (`Actor.SetActorTickEnabled` _currentbulletinarray true)
        (`Actor.K2_SetActorTransform` _currentbulletinarray (`.Origin` (break `BulletData` (`local.bulletData`))) false false)
        (`/Game/Blueprints/BasicBullet.FireProjectile` _currentbulletinarray (`local.bulletData`))
        (return (`local.CurrentBulletInArray`)))))
  (`self.DisableMe` (`self.OldestBullet`))
  (set `self.LongestLifetime` 0.0)
  (`Actor.SetActorHiddenInGame` _oldestbullet false)
  (`Actor.SetActorTickEnabled` _oldestbullet true)
  (`Actor.K2_SetActorTransform` _oldestbullet (`.Origin` (break `BulletData` (`local.bulletData`))) false false)
  (`/Game/Blueprints/BasicBullet.FireProjectile` (`self.OldestBullet`) (`local.bulletData`))
  (return (`self.OldestBullet`)))