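; SpaceDancer is the player-controlled flyer in a shmup, with thruster audio, animation-driven strafing and switchable minigun, missile and shotgun weapons.
; Axis input ramps clamped move values that feed the anim instance and Tick, which decelerates them and interpolates Position along its local axes.
; Camera and body smoothly turn toward a look target as the camera trails behind.
; Look input, gated by LMBPressed (setters unwired), rotates CameraRoot and publishes player location to the GameInstance.
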(event `self.ReceiveBeginPlay`
  (bind _position (`self.Position`))
  (`FMODBlueprintStatics.PlayEventAttached` "/Game/FMOD/Events/Main_Thruster.Main_Thruster" _position "None" (`SceneComponent.K2_GetComponentLocation` _position) "KeepWorldPosition" false true false)
  (`self.K2_AttachToActor` (`GameplayStatics.GetPlayerController` 0) self "None" "KeepWorld" "KeepWorld" "KeepRelative" false)
  (bind _asdancer_anim_print (cast `/Game/Blueprints/DancerAnimPrint` (`SkeletalMeshComponent.GetAnimInstance` (`self.SkeletalMesh`))))
  (set `self.DancerAnims` _asdancer_anim_print))

(event `Key|LeftMouseButton`
  (params (Key :type "Key Structure")))

(event `InputAxis|uP`
  (params (AxisValue :type "Float (single-precision)"))
  (bind _modifiedval (`self.SmoothUpSpeed` (`self.upMoveVal`) AxisValue (`self.acceleration`)))
  (bind _output_get (set `self.upMoveVal` _modifiedval))
  (set `/Game/Blueprints/DancerAnimPrint.Up` _output_get (`self.DancerAnims`)))

(event `InputAxis|Right`
  (params (AxisValue :type "Float (single-precision)"))
  (bind _modifiedval (`self.SmoothUpSpeed` (`self.rightMoveVal`) AxisValue (`self.acceleration`)))
  (bind _output_get (set `self.rightMoveVal` _modifiedval))
  (set `/Game/Blueprints/DancerAnimPrint.StrafeRight` _output_get (`self.DancerAnims`)))

(event `InputAxis|Turn`
  (params (AxisValue :type "Float (single-precision)"))
  (if (`self.LMB Pressed`)
    (`SceneComponent.K2_SetWorldRotation` (`self.cameraRoot`) (`KismetMathLibrary.MakeRotator` 0.0 (`self.currentPitch`) (+ (* AxisValue (`self.hortizontalLookSpeed`)) (.yaw (`SceneComponent.K2_GetComponentRotation` (`self.cameraRoot`))))) false false :!label _label)
    (bind _asshmup_game_instance (cast `/Game/Blueprints/ShmupGameInstance` (`GameplayStatics.GetGameInstance`)))
    (set `/Game/Blueprints/ShmupGameInstance.Player World Location` (`SceneComponent.K2_GetComponentLocation` (`self.Position`)) _asshmup_game_instance)))

(event `InputAxisKey|MouseX`
  (params (AxisValue :type "Float (single-precision)")))

(event `InputAxis|Forward`
  (params (AxisValue :type "Float (single-precision)"))
  (bind _modifiedval (`self.SmoothUpSpeed` (`self.forwardMoveVal`) AxisValue (`self.acceleration`)))
  (bind _output_get (set `self.forwardMoveVal` _modifiedval))
  (set `/Game/Blueprints/DancerAnimPrint.Forward` _output_get (`self.DancerAnims`)))

(event `InputAxisKey|MouseY`
  (params (AxisValue :type "Float (single-precision)")))

(event `self.ReceiveTick`
  (params (DeltaSeconds :type "Float (single-precision)"))
  (bind _returnvalue (`SceneComponent.K2_GetComponentLocation` (`self.Position`)))
  (bind _returnvalue_2 (`SceneComponent.K2_GetComponentLocation` (`self.Position`)))
  (bind _returnvalue_3 (`SceneComponent.K2_GetComponentLocation` (`self.Position`)))
  (if (== (stale `InputAxis|uP` AxisValue) 0.0)
    (set `self.movingUp` false)
    (else
      (set `self.movingUp` true)))
  (if (== (stale `InputAxis|Right` AxisValue) 0.0)
    (set `self.movingRIght` false)
    (else
      (set `self.movingRIght` true)))
  (if (== (stale `InputAxis|Forward` AxisValue) 0.0)
    (set `self.movingForward` false)
    (else
      (set `self.movingForward` true)))
  (bind _modifiedspeed (`self.SmoothDownSpeed` (`self.movingForward`) (`self.forwardMoveVal`)))
  (set `self.forwardMoveVal` _modifiedspeed)
  (bind _modifiedspeed_2 (`self.SmoothDownSpeed` (`self.movingUp`) (`self.upMoveVal`)))
  (set `self.upMoveVal` _modifiedspeed_2)
  (bind _modifiedspeed_3 (`self.SmoothDownSpeed` (`self.movingRIght`) (`self.rightMoveVal`)))
  (set `self.rightMoveVal` _modifiedspeed_3)
  (`PlayerController.SetAudioListenerOverride` :`self` (`GameplayStatics.GetPlayerController` 0) :`Location` (`SceneComponent.K2_GetComponentLocation` (`self.Position`)))
  (set `self.deltaTime` DeltaSeconds)
  (`SceneComponent.K2_SetWorldLocation` (`self.Position`) (`KismetMathLibrary.VInterpTo` _returnvalue_2 (+ _returnvalue_2 (* (`KismetMathLibrary.GetRightVector` (`SceneComponent.K2_GetComponentRotation` (`self.Position`))) (* (`self.rightMoveVal`) (`self.moveSpeed`)))) (`self.deltaTime`) (`self.moveMult`)) false false)
  (`SceneComponent.K2_SetWorldLocation` (`self.Position`) (`KismetMathLibrary.VInterpTo` _returnvalue_3 (+ _returnvalue_3 (* (`SceneComponent.GetForwardVector` (`self.Position`)) (* (`self.forwardMoveVal`) (`self.moveSpeed`))) (0.0 0.0 0.0)) (`self.deltaTime`) (`self.moveMult`)) false false)
  (`SceneComponent.K2_SetWorldLocation` (`self.Position`) (`KismetMathLibrary.VInterpTo` _returnvalue (+ (* (`SceneComponent.GetUpVector` (`self.Position`)) (* (`self.upMoveVal`) (`self.moveSpeed`))) _returnvalue) (`self.deltaTime`) (`self.moveMult`)) false false)
  (`SceneComponent.K2_SetWorldLocation` (`self.cameraRoot`) (`SceneComponent.K2_GetComponentLocation` (`self.Position`)) false false)
  (`self.SmoothLookAt` (`self.Camera`) (`self.CameraLookTarget`) (`self.cameraLookSpeed`))
  (`self.SmoothLookAt` (`self.Position`) (`self.CameraLookTarget`) (`self.dancerLookSpeed`))
  (`SceneComponent.K2_SetWorldLocation` (`self.Camera`) (`KismetMathLibrary.VInterpTo` (`SceneComponent.K2_GetComponentLocation` (`self.Camera`)) (`SceneComponent.K2_GetComponentLocation` (`self.CameraPosTarget`)) (`self.deltaTime`) (`self.cameraMoveSpeed`)) false false))

(event `InputAxis|LookUp`
  (params (AxisValue :type "Float (single-precision)"))
  (bind _currentpitch (`self.currentPitch`))
  (bind _minpitch (`self.minPitch`))
  (bind _maxpitch (`self.maxPitch`))
  (bind _result (`/Engine/EditorBlueprintResources/StandardMacros.NegateFloat` AxisValue)
    (:`  `
      (if (`self.LMB Pressed`)
        (bind _output_get (set `self.currentPitch` (+ _currentpitch (* _result (`self.verticalLookSpeed`)))))
        (if (>= _currentpitch _minpitch)
          (if (<= _currentpitch _maxpitch)
            (goto _label)
            (else
              (set `self.currentPitch` _maxpitch)))
          (else
            (set `self.currentPitch` _minpitch)))))))

(event `InputAction|Fire`
  (params (Key :type "Key Structure"))
  (bind _dancerfire (`self.DancerFire`))
  (:`Pressed`
    (set `/Game/Blueprints/DancerFire.FireWeap1` true _dancerfire))
  (:`Released`
    (set `/Game/Blueprints/DancerFire.FireWeap1` false _dancerfire)))

(event `InputAction|Fire2`
  (params (Key :type "Key Structure")))

(event `InputAction|Switch 1`
  (params (Key :type "Key Structure"))
  (bind _dancerfire (`self.DancerFire`))
  (:`Pressed`
    (set `/Game/Blueprints/DancerFire.currentWeapon1` (`/Game/Blueprints/DancerFire.DoubleMinigun` _dancerfire) _dancerfire)
    (`SceneComponent.SetVisibility` (`self.LMinigun`) true false)
    (`SceneComponent.SetVisibility` (`self.RMinigun`) true false)
    (`SceneComponent.SetVisibility` (`self.Missiles`) false false)
    (set `/Game/Blueprints/DancerFire.Default Fire Origins` (`/Game/Blueprints/DancerFire.MinigunFireOrigins` _dancerfire) _dancerfire)))

(event `InputAction|Switch 2`
  (params (Key :type "Key Structure"))
  (bind _dancerfire (`self.DancerFire`))
  (:`Pressed`
    (set `/Game/Blueprints/DancerFire.currentWeapon1` (`/Game/Blueprints/DancerFire.DoubleMissile` _dancerfire) _dancerfire)
    (`SceneComponent.SetVisibility` (`self.Missiles`) true false)
    (`SceneComponent.SetVisibility` (`self.LMinigun`) false false)
    (`SceneComponent.SetVisibility` (`self.RMinigun`) false false)
    (set `/Game/Blueprints/DancerFire.Default Fire Origins` (`/Game/Blueprints/DancerFire.MissileFireOrigins` _dancerfire) _dancerfire)))

(event `InputAction|Switch 3`
  (params (Key :type "Key Structure"))
  (bind _dancerfire (`self.DancerFire`))
  (:`Pressed`
    (set `/Game/Blueprints/DancerFire.currentWeapon1` (`/Game/Blueprints/DancerFire.SingleShotgun` _dancerfire) _dancerfire)
    (set `/Game/Blueprints/DancerFire.Default Fire Origins` (`/Game/Blueprints/DancerFire.ShotgunFireOrigins` _dancerfire) _dancerfire)))

(fn `SmoothDownSpeed`
  (params (movingCondition :type Boolean) (moveVal :type "Float (double-precision)"))
  (returns (modifiedSpeed :type "Float (double-precision)"))
  (if movingCondition
    (return moveVal)
    (elif (`KismetMathLibrary.NearlyEqual_FloatFloat` (`local.moveVal`) 0.0 0.05)
      (return 0.0)
      (elif (> (`local.moveVal`) 0.0)
        (return (- (`local.moveVal`) (`self.deceleration`)))
        (else
          (return (+ (`local.moveVal`) (`self.deceleration`))))))))

(fn `SmoothLookAt`
  (params (`Looking Object` :type "SceneComponent Object Reference") (`Look Target` :type "SceneComponent Object Reference") (LookSpeed :type "Float (double-precision)"))
  (locals (NewLocalVar_0 :type "SceneComponent Object Reference") (NewLocalVar_1 :type "SceneComponent Object Reference"))
  (`SceneComponent.K2_SetWorldRotation` `Look Target` (`KismetMathLibrary.RInterpTo` (`SceneComponent.K2_GetComponentRotation` `Looking Object`) (`KismetMathLibrary.FindLookAtRotation` (`SceneComponent.K2_GetComponentLocation` `Looking Object`) (`SceneComponent.K2_GetComponentLocation` `Look Target`)) (`self.deltaTime`) LookSpeed) false false)
  (`SceneComponent.K2_SetWorldRotation` `Looking Object` (`KismetMathLibrary.RInterpTo` (`SceneComponent.K2_GetComponentRotation` `Looking Object`) (`KismetMathLibrary.FindLookAtRotation` (`SceneComponent.K2_GetComponentLocation` `Looking Object`) (`SceneComponent.K2_GetComponentLocation` `Look Target`)) (`self.deltaTime`) LookSpeed) false false))

(fn `SmoothUpSpeed`
  (params (moveVal :type "Float (double-precision)") (axisVal :type "Float (double-precision)") (acceleration :type "Float (double-precision)"))
  (returns (modifiedVal :type "Float (double-precision)"))
  (bind _returnvalue (+ (* axisVal acceleration) (`local.moveVal`)))
  (if (>= _returnvalue 1.0)
    (return 1.0)
    (elif (<= _returnvalue -1.0)
      (return -1.0)
      (else
        (return _returnvalue)))))

(fn `UserConstructionScript`)